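; Behavior tree service that finds a climbable for an AI creature on each tick.
; It sphere-overlaps WorldDynamic objects around a blackboard origin actor, filtered to ClimbableMarker.
; The first marker found, not necessarily the nearest, is written to the blackboard, along with its climb start as the target location and its position as the climb destination.
; With no overlap, it clears only the climbable key, leaving both locations unchanged.
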(event EventTick
  (params (OwnerActor :type Actor%20Object%20Reference) (DeltaSeconds :type Float%20%28single-precision%29))
  (if (!= (Variables|Default|GetAIController) 0)
    _
    (else
      (bind _asaicontroller (Utilities|Casting|CastToAIController OwnerActor))
      (Variables|Default|SetAIController _asaicontroller)))
  (bind (_outactors _returnvalue) (Class|KismetSystemLibrary|SphereOverlapActorsNEW (Transformation|GetActorLocation (AI|BehaviorTree|GetBlackboardValueasActor (Variables|Default|GetSphereOriginActor))) (Variables|Default|GetSphereCheckRadius) (Utilities|Array|MakeArray "ObjectTypeQuery2") "/Game/Blueprints/Objects/LevelWidgets/ClimbableMarker.ClimbableMarker_C"))
  (if _returnvalue
    (bind _array_element (Utilities|Array|ForEachLoopwithBreak _outactors :!label _label)
      (:LoopBody
        (bind _asclimbable_marker (Utilities|Casting|CastToClimbableMarker _array_element))
        (Class|BTFunctionLibrary|SetBlackboardValueasObject (Variables|Default|GetClimbableToSet) _asclimbable_marker)
        (bind _climb_start_location (Default|GetClimbStartLocation _asclimbable_marker))
        (AI|BehaviorTree|SetBlackboardValueasVector (Variables|Default|GetTargetLocation) _climb_start_location)
        (AI|BehaviorTree|SetBlackboardValueasVector (Variables|Default|GetClimbDestination) (Transformation|GetActorLocation _asclimbable_marker))
        (goto _label Break)))
    (else
      (Class|BTFunctionLibrary|SetBlackboardValueasObject (Variables|Default|GetClimbableToSet)))))