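; FaceActor is an unfinished behavior tree node, apparently meant to turn an AI-controlled creature toward the blackboard actor ActorToFace.
; On Tick it casts the owner to AIController and caches it if not already set, and does nothing else.
; The pawn rotation call is unreachable and holds a zero rotation, and the target's location and rotation lookups are unused.
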(event EventTick
  (params (OwnerActor :type Actor%20Object%20Reference) (DeltaSeconds :type Float%20%28single-precision%29))
  (if (not (!= (Variables|Default|GetAIController) 0))
    (bind _asaicontroller (Utilities|Casting|CastToAIController OwnerActor))
    (Variables|Default|SetAIController _asaicontroller)))