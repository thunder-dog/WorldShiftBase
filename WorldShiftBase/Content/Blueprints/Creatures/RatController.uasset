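; RatController is the AI controller for rat creatures, handing the rat's owning player to its behavior tree.
; Shortly after BeginPlay, it casts the controlled pawn to the rat class, gets its owning player, and stores it in the RatBoard blackboard's Player key.
; It then runs RatTree, or prints an error naming the pawn if the cast fails.
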(event EventBeginPlay
  (bind _returnvalue (Pawn|GetControlledPawn))
  (Utilities|FlowControl|Delay 0.1)
  (bind _asrat (Utilities|Casting|CastTorat _returnvalue)
    (:then
      (bind _owningplayer (Default|GetOwningPlayer _asrat))
      (bind _output_get (Variables|Default|SetOwningPlayer _owningplayer))
      (bind _blackboardcomponent (Class|AIController|UseBlackboard "/Game/Blueprints/Creatures/RatBoard.RatBoard"))
      (AI|Components|Blackboard|SetValueasObject _blackboardcomponent (Variables|Default|GetPlayer) _output_get)
      (AI|RunBehaviorTree "/Game/Blueprints/Creatures/RatTree.RatTree"))
    (:CastFailed
      (Development|PrintString (Utilities|String|Append ": AI Rat Controller not attached to rat actor class" (Utilities|GetObjectName _returnvalue)) false))))

(event EventTick
  (params (DeltaSeconds :type Float%20%28single-precision%29)))

(fn ConstructionScript)