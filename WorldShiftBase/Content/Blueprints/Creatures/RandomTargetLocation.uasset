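; Behavior Tree task for rat AI that writes a random target location around an origin actor to the Blackboard.
; On tick, it caches the owner as a RatController and optionally stops its current movement.
; It picks a flat random offset within a square, rotates it by the origin actor's rotation, adds that actor's location, then finishes successfully.
; A failed controller cast exits without finishing the task.
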(event EventTick
  (params (OwnerActor :type Actor%20Object%20Reference) (DeltaSeconds :type Float%20%28single-precision%29))
  (bind _randomorigin (Variables|Default|GetRandomOrigin))
  (bind _randomdistancesize (Variables|Default|GetRandomDistanceSize))
  (bind _returnvalue (AI|BehaviorTree|GetBlackboardValueasActor _randomorigin))
  (bind _returnvalue_2 (* _randomdistancesize -1.0))
  (if (!= (Variables|Default|GetAI_Controller) 0)
    _
    (else
      (bind _asrat_controller (Utilities|Casting|CastToRatController OwnerActor))
      (Variables|Default|SetAI_Controller _asrat_controller)))
  (if (Variables|Default|GetInterruptCurrentMovement)
    (AI|Navigation|StopMovement (Variables|Default|GetAI_Controller)))
  (AI|BehaviorTree|SetBlackboardValueasVector (Variables|Default|GetTargetLocationKey) (+ (Math|Vector|RotateVector (Math|Vector|MakeVector (Math|Random|RandomFloatinRange _returnvalue_2 _randomdistancesize) (Math|Random|RandomFloatinRange _returnvalue_2 _randomdistancesize) 0.0) (Transformation|GetActorRotation _returnvalue)) (Transformation|GetActorLocation _returnvalue)))
  (AI|BehaviorTree|FinishExecute true))