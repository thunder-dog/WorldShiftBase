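; AI-controlled rat creature tied to an owning player, who can pick it up or store it as an inventory item.
; It teleports behind the player when it strays too far or the player's world-rip finish dispatch fires.
; Grabbing toggles capsule physics, drives a physics handle and sets a picked-up Blackboard flag.
; AI logic can be paused, and storing adds the item to the owner's inventory and destroys the actor.
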(event Custom|DetectWorldRip
  (CallFunction|TeleportRatBehindPlayer))

(event EventTeleportRatBehindPlayer
  (bind _owningplayer (Variables|Default|GetOwningPlayer))
  (bind _returnvalue (Transformation|GetActorRotation _owningplayer))
  ;[1 1 1] Move  behind player
  (bind _transform (Class|RatInterface|GetCameraTransform(Message) _owningplayer))
  (Transformation|SetActorLocationAndRotation (+ (* (* (Math|Vector|GetForwardVector (.Rotation (Math|Transform|BreakTransform _transform))) -2e+02) (Utilities|Absolute(Vector) (- (Math|Vector|GetUpVector _returnvalue) 1.0))) (Transformation|GetActorLocation _owningplayer)) _returnvalue false true))

(event EventStartStopLogic
  (params (Flag :type Boolean))
  (bind _aicontroller (Variables|Default|GetAIController))
  (bind _braincomponent (Variables|/Script/AIModule.AIController|GetBrainComponent _aicontroller))
  ;[1 1 1] Logic on and off
  (if Flag
    (Class|BrainComponent|RestartLogic _braincomponent)
    (else
      (AI|Logic|StopLogic _braincomponent "Requested by function in controlled pawn"))))

(event EventStartGrab
  (params (GrabLocation :type Vector) (NewOwner :type Actor%20Object%20Reference) (NewInInventory :type Boolean) (GrabRotation :type Rotator :default "0, 0, 0"))
  (bind _capsulecomponent (Variables|Collision|GetCapsuleComponent))
  (Physics|SetSimulatePhysics _capsulecomponent true)
  (Class|PhysicsHandleComponent|GrabComponent (Variables|Default|GetPhysicsHandle) _capsulecomponent "None" GrabLocation false)
  (AI|Components|Blackboard|SetValueasBool (Variables|Default|GetBlackBoard) (Variables|Default|GetPickedUpName) true))

(event EventSetHoldingLocRot
  (params (HoldLocation :type Vector) (HoldRotation :type Rotator :default "0, 0, 0"))
  (Physics|Components|PhysicsHandle|SetTargetLocation (Variables|Default|GetPhysicsHandle) HoldLocation))

(event EventStopGrab
  (Physics|Components|PhysicsHandle|ReleaseComponent (Variables|Default|GetPhysicsHandle))
  (Physics|SetSimulatePhysics (Variables|Collision|GetCapsuleComponent) false)
  (AI|Components|Blackboard|SetValueasBool (Variables|Default|GetBlackBoard) (Variables|Default|GetPickedUpName) false))

(event EventKillandAddItem
  (params (Owner :type Actor%20Object%20Reference))
  (if (== (Variables|Default|GetOwningPlayer) Owner)
    (Class|UsableItemInterface|AddItemtoInventory(Message) Owner (Utilities|RatID) "" 0 "1.000000,1.000000,1.000000" "1.000000,1.000000,1.000000")
    (Actor|DestroyActor)))

(event EventBeginPlay
  (Variables|Default|SetItemID (Utilities|RatID))
  (Utilities|FlowControl|Delay 0.2)
  (bind _returnvalue (AI|GetAIController self))
  (bind _output_get (Variables|Default|SetAIController _returnvalue))
  (Variables|Default|SetBlackBoard (AI|GetBlackboard _output_get))
  (bind _asplayer_dummy (Utilities|Casting|CastToPlayerDummy (Variables|Default|GetOwningPlayer)))
  (EventDispatchers|BindEventtoWorldRipFinishDispatch _asplayer_dummy (delegate Custom|DetectWorldRip)))

(event EventActorBeginOverlap
  (params (OtherActor :type Actor%20Object%20Reference)))

(event EventTick
  (params (DeltaSeconds :type Float%20%28single-precision%29))
  (if (> (Math|Vector|VectorLength (- (Transformation|GetActorLocation) (Transformation|GetActorLocation (Variables|Default|GetOwningPlayer)))) 1e+03)
    (CallFunction|TeleportRatBehindPlayer)))

(fn ConstructionScript)

(fn SetOwningPlayer
  (params (NewOwningPlayer :type Actor%20Object%20Reference))
  (Variables|Default|SetOwningPlayer NewOwningPlayer)
  (return))

(fn GetOwningPlayer
  (return (Variables|Default|GetOwningPlayer)))

(fn GetCameraTransform
  (return ""))

(fn GetCanStore
  (return true))

(fn GetItemMesh
  (return 0))

(fn GetParams
  (return (Utilities|RatID) "" 0 "1.000000,1.000000,1.000000" "1.000000,1.000000,1.000000" false))