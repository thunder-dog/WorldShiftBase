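; Pickupable item actor that can be carried with a physics handle and returned to its owner's inventory.
; Grabbing records the owner and drives the mesh toward a hold transform, shrinking it and ignoring physics bodies when held in inventory.
; Dropping restores size and collision, then after a retriggerable delay a storable, unheld item sends its data to the owner and destroys itself.
; PingOff launches the mesh with a random impulse.
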(event EventKillandAddItem
  (Class|UsableItemInterface|AddItemtoInventory(Message) (Variables|Default|GetItemOwner) (Variables|ItemData|GetItemID) (Variables|ItemData|GetItemName) (Variables|ItemData|GetItemMesh) (Variables|ItemData|GetRealScale) (Variables|ItemData|GetInventoryScale))
  (Actor|DestroyActor))

(event EventMakeBigger
  (Transformation|SetActorScale3D (Variables|ItemData|GetRealScale))
  (Collision|SetCollisionResponsetoChannel (Variables|Components|GetStaticMesh) "ECC_PhysicsBody" "ECR_Block"))

(event EventStartGrab
  (params (GrabLocation :type Vector) (NewOwner :type Actor%20Object%20Reference) (NewInInventory :type Boolean))
  (Class|PhysicsHandleComponent|GrabComponent (Variables|Default|GetPhysicsHandle) (Variables|Components|GetStaticMesh) "None" GrabLocation true)
  (Variables|Default|SetInitialGrabRotation (Transformation|GetWorldRotation (Variables|Components|GetStaticMesh)))
  (Variables|Default|SetCurrentlyHeld true)
  (Variables|Default|SetItemOwner NewOwner)
  (Variables|Default|SetInInventory NewInInventory)
  (if (Variables|Default|GetInInventory)
    (Transformation|SetActorScale3D (Variables|ItemData|GetInventoryScale))
    (Collision|SetCollisionResponsetoChannel (Variables|Components|GetStaticMesh) "ECC_PhysicsBody" "ECR_Ignore")
    (else
      (Transformation|SetActorScale3D (Variables|ItemData|GetRealScale))
      (Collision|SetCollisionResponsetoChannel (Variables|Components|GetStaticMesh) "ECC_PhysicsBody" "ECR_Block"))))

(event EventSetHoldingLocRot
  (params (HoldLocation :type Vector) (HoldRotation :type Rotator))
  (bind _initialgrabrotation (Variables|Default|GetInitialGrabRotation))
  (Class|PhysicsHandleComponent|SetTargetLocationandRotation (Variables|Default|GetPhysicsHandle) HoldLocation (Math|Rotator|CombineRotators (Math|Rotator|Delta(Rotator) HoldRotation _initialgrabrotation) _initialgrabrotation)))

(event EventStopGrab
  (Physics|Components|PhysicsHandle|ReleaseComponent (Variables|Default|GetPhysicsHandle))
  (CallFunction|MakeBigger)
  (Collision|SetCollisionResponsetoChannel (Variables|Components|GetStaticMesh) "ECC_PhysicsBody" "ECR_Block")
  (Variables|Default|SetCurrentlyHeld false)
  (Utilities|FlowControl|RetriggerableDelay (Variables|Default|GetLifeAfterDrop))
  (if (and (Variables|ItemData|GetCanBeStored) (Math|Boolean|NotEqual(Boolean) (Variables|Default|GetCurrentlyHeld) true))
    (Class|UsableItemInterface|AddItemtoInventory(Message) (Variables|Default|GetItemOwner) (Variables|ItemData|GetItemID) (Variables|ItemData|GetItemName) (Variables|ItemData|GetItemMesh) (Variables|ItemData|GetRealScale) (Variables|ItemData|GetInventoryScale))
    (Actor|DestroyActor)))

(event EventPingOff
  (Physics|AddImpulse (Variables|Components|GetStaticMesh) (* (Math|Random|RandomUnitVector) (Math|Random|RandomFloatinRange 2.5e+03 5e+03)) "None" false))

(fn ConstructionScript
  (Components|StaticMesh|SetStaticMesh (Variables|Components|GetStaticMesh) (Variables|ItemData|GetItemMesh))
  (Transformation|SetActorScale3D (Variables|ItemData|GetRealScale)))

(fn GetIemMesh)

(fn GetCanStore
  (return (Variables|ItemData|GetCanBeStored)))

(fn GetItemMesh
  (return (Variables|Components|GetStaticMesh)))

(fn GetParams
  (return (Variables|ItemData|GetItemID) (Variables|ItemData|GetItemName) (Variables|ItemData|GetItemMesh) (Variables|ItemData|GetRealScale) (Variables|ItemData|GetInventoryScale)))