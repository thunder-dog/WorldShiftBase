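; Pullable object Blueprint that plays a one-shot animation on a configurable skeletal mesh when pulled.
; The Pulled event sets a Fired guard and waits out a cooldown, then re-arms unless FireOnce is set.
; PullablePulled is called after the cooldown, not at the moment of the pull.
; The construction script applies the chosen mesh and toggles its collision from UseObjectCollision.
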(event EventBeginPlay)

(event EventActorBeginOverlap
  (params (OtherActor :type Actor%20Object%20Reference)))

(event EventTick
  (params (DeltaSeconds :type Float%20%28single-precision%29)))

(event EventPulled
  (params (PullPoint :type Vector :default "0, 0, 0"))
  (if (not (Variables|Default|GetFired))
    (Components|Animation|PlayAnimation (Variables|Default|GetSkeletalMesh) (Variables|Default|GetPullAnimation) false)
    (Variables|Default|SetFired true)
    (Utilities|FlowControl|Delay (Variables|Default|GetCooldown))
    (if (Variables|Default|GetFireOnce)
      _
      (else
        (Variables|Default|SetFired false)))
    (Default|CallPullablePulled)))

(fn ConstructionScript
  (bind _skeletalmesh (Variables|Default|GetSkeletalMesh))
  (Class|SkinnedMeshComponent|SetSkeletalMesh (Variables|Default|GetSkeletalMesh) (Variables|Default|GetMesh))
  (if (Variables|Default|GetUseObjectCollision)
    (Collision|SetCollisionEnabled _skeletalmesh "QueryAndPhysics")
    (else
      (Collision|SetCollisionEnabled _skeletalmesh "NoCollision"))))