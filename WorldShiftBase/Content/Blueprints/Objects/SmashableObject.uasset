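; Smashable destructible prop that the player breaks with smashing fists, with its mesh set in the construction script and an option to start asleep.
; Each hit from a PlayerSmashingFist applies point damage and lowers Health by a fraction based on HitsToKill.
; At zero health it switches to the Destructible collision type, takes a velocity-change impulse from the fist's move delta, and destroys itself after a delay.
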(event OnComponentHit(Destructible)
  (params (OtherActor :type Actor%20Object%20Reference) (OtherComp :type Primitive%20Component%20Object%20Reference) (NormalImpulse :type Vector :default "0, 0, 0") (Hit :type Hit%20Result%20Structure%20%28by%20ref%29))
  (bind (_bblockinghit _binitialoverlap _time _location _impactpoint _normal _impactnormal _physmat _hitactor _hitcomponent) (Collision|BreakHitResult Hit))
  (bind _hitstokill (Variables|Default|GetHitsToKill))
  (bind _returnvalue (/ 1.0 _hitstokill))
  (bind _asplayer_smashing_fist (Utilities|Casting|CastToPlayerSmashingFist OtherActor))
  (bind _movedelta (Default|GetMoveDelta _asplayer_smashing_fist))
  (Game|Damage|ApplyPointDamage _hitactor _returnvalue _impactpoint Hit 0 0 "/Script/Engine.DamageType")
  (bind _newhealth (CallFunction|DecreaseHealth _returnvalue))
  (if (<= _newhealth 0.0)
    (Physics|AddImpulse _hitcomponent _movedelta "None" true)
    (Collision|SetCollisionObjectType (Variables|Default|GetDestructible) "ECC_Destructible")
    (Utilities|FlowControl|Delay 7.5)
    (Actor|DestroyActor)))

(event EventBeginPlay
  (if (Variables|Default|GetStartSleeping)
    (Class|PrimitiveComponent|PutRigidBodytoSleep (Variables|Default|GetDestructible) "None")))

(event EventActorBeginOverlap
  (params (OtherActor :type Actor%20Object%20Reference)))

(event EventTick
  (params (DeltaSeconds :type Float%20%28single-precision%29)))

(fn ConstructionScript
  (Class|DestructibleComponent|SetDestructibleMesh (Variables|Default|GetDestructible) (Variables|Default|GetMesh)))

(fn DecreaseHealth
  (params (HitAmount :type Float%20%28single-precision%29))
  (bind _output_get (LocalVariables|SetTempHealth (Variables|Default|GetHealth)))
  (bind _output_get_2 (Variables|Default|SetHealth (- _output_get HitAmount)))
  (return _output_get_2))