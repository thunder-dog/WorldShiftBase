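; DeformingWorldSegment is a piece of the level that visually deforms when the world shifts or unshifts.
; WorldShifter and WorldUnshifter each play a one-shot deform animation on its skeletal mesh.
; On BeginPlay it reads the shift state from PlayerDummy actors and runs WorldShifter if the world is already shifted.
; The construction script applies the configured mesh and toggles its collision through UseMeshCollision.
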(event Custom|WorldShifter
  ;[1 1 1] Worldshifting
  (Components|Animation|PlayAnimation (Variables|Default|GetSkeletalMesh) (Variables|Default|GetWorldShiftDeform) false))

(event Custom|WorldUnshifter
  ;[1 1 1] Worldshifting
  (Components|Animation|PlayAnimation (Variables|Default|GetSkeletalMesh) (Variables|Default|GetWorldUnshiftDeform) false))

(event EventBeginPlay
  ;[1 1 1] Check to see if world is shifted on load and shift yourself if it is
  (bind _outactors (Actor|GetAllActorsOfClass "/Game/Blueprints/Player/PlayerDummy.PlayerDummy_C"))
  (for _array_element _outactors
    (bind _worldshiftstate (Default|GetWorldShiftState _array_element))
    (if _worldshiftstate
      (CallFunction|WorldShifter))))

(event EventActorBeginOverlap
  (params (OtherActor :type Actor%20Object%20Reference)))

(event EventTick
  (params (DeltaSeconds :type Float%20%28single-precision%29)))

(fn ConstructionScript
  (bind _skeletalmesh (Variables|Default|GetSkeletalMesh))
  (Class|SkinnedMeshComponent|SetSkeletalMesh (Variables|Default|GetSkeletalMesh) (Variables|Default|GetMesh))
  (if (Variables|Default|GetUseMeshCollision)
    (Collision|SetCollisionEnabled _skeletalmesh "QueryAndPhysics")
    (else
      (Collision|SetCollisionEnabled _skeletalmesh "NoCollision"))))