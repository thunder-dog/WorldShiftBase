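; Player component for WorldRip, a ranged teleport onto floors, walls or ceilings.
; Start line-traces from the camera and spawns a preview at the target; finish derives the surface's up axis and plays a sphere effect before teleporting the owner after a delay.
; During the rip, Tick moves a cube capture at the destination with the player's movement, masked along the new up axis.
; Reference and dynamic-material setup is disconnected from BeginPlay.
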(event Custom|WorldRipStart
  (bind _cameracomponent (Variables|Components|GetCameraComponent))
  (bind _returnvalue (Transformation|GetWorldLocation _cameracomponent))
  (if (not (Variables|Default|GetWorldRipInProgress))
    (bind _outhit (Collision|LineTraceForObjects _returnvalue (+ _returnvalue (* (Math|Vector|GetForwardVector (Transformation|GetWorldRotation _cameracomponent)) (Variables|Default|GetWorldRipRange))) (Utilities|Array|MakeArray "ObjectTypeQuery7") false 0 "None"))
    (Utilities|Casting|CastTo (.HitActor (Collision|BreakHitResult _outhit))
      (:then
        (Variables|Default|SetTargetFloorSurface 0)
        (bind _targetfloororigin (CallFunction|GetTargetFloorOrigin))
        (bind _output_get (Variables|Default|SetTargetLocation _targetfloororigin))
        (bind _returnvalue_2 (Game|SpawnActorfromClass (Variables|Default|GetPreviewActor) (Math|Transform|MakeTransform _output_get "0.0,0.0,0.0" "1,1,1") "AlwaysSpawn" 0 0))
        (Variables|Default|SetActivePreviewModel _returnvalue_2)
        (Variables|Default|SetWorldRipPrep true)
        (Variables|Default|SetActivationLocation (Transformation|GetWorldLocation (Variables|Default|GetCapsuleComponent))))
      (:CastFailed
        (Development|PrintString "Target does not match WorldRipSurface class")))))

(event Custom|WorldRipFinish
  (bind _returnvalue (Components|GetOwner))
  (bind _worldripsphere (Variables|Default|GetWorldRipSphere))
  (bind _targetlocation (Variables|Default|GetTargetLocation))
  (bind _returnvalue_2 (Transformation|GetActorLocation _returnvalue))
  (bind _returnvalue_3 (- _targetlocation _returnvalue_2))
  (bind _returnvalue_4 (Math|Vector|Normalize _returnvalue_3))
  (bind (_x _y _z) (Math|Vector|BreakVector _returnvalue_4))
  (if (Variables|Default|GetWorldRipPrep)
    (Variables|Default|SetWorldRipInProgress true)
    (Variables|Default|SetWorldRipPrep false)
    (Actor|DestroyActor (Variables|Default|GetActivePreviewModel))
    (Development|PrintString "WorldRip in progress!")
    (bind _newfloor (CallFunction|GetNewFloor))
    (switch Utilities|FlowControl|Switch|Switchon _newfloor
      (:NewEnumerator0
        (Variables|Default|SetTargetUp "0,0.000000,1.000000"))
      (:NewEnumerator1
        (Variables|Default|SetTargetUp "0, 0,-1.000000"))
      (:NewEnumerator2
        (Variables|Default|SetTargetUp "1.000000, 0, 0"))
      (:NewEnumerator3
        (Variables|Default|SetTargetUp "-1.000000, 0, 0"))
      (:NewEnumerator4
        (Variables|Default|SetTargetUp "0,1.000000, 0"))
      (:NewEnumerator5
        (Variables|Default|SetTargetUp "0,-1.000000, 0")))
    ;[1 1 1] Make Target Camera Location
    (Development|PrintString "get cam height was here")
    (Transformation|SetWorldLocationAndRotation (Variables|Default|GetWorldRipCubeCapture) (+ _targetlocation (* (Variables|Default|GetTargetUp) 0.0)) "0, 0, 0" false true)
    (Rendering|Material|SetVectorParameterValue (Variables|Default|GetSphereMaterial) "TargetPointer" (Utilities|Struct|MakeLinearColor _x _y _z 0.0) :!class /Script/Engine.MaterialInstanceDynamic)
    (Components|Animation|PlayAnimation _worldripsphere 0 false)
    (Utilities|FlowControl|Delay 0.1)
    (Rendering|SetVisibility _worldripsphere true false)
    (Utilities|FlowControl|Delay (Variables|Default|GetWorldRipDuration))
    (Transformation|SetActorLocationAndRotation (Components|GetOwner) (+ (* (Variables|Default|GetTargetUp) (Components|Capsule|GetScaledCapsuleHalfHeight (Variables|Default|GetCapsuleComponent))) (* (- (Transformation|GetWorldLocation (Variables|Default|GetCapsuleComponent)) (Variables|Default|GetActivationLocation)) (Utilities| (- (Utilities| (Variables|Default|GetTargetUp)) "1.000000,1.000000,1.000000"))) (Variables|Default|GetTargetLocation)) "0, 0, 0" false true)
    (Rendering|SetVisibility (Variables|Default|GetWorldRipSphere) false false)
    (Variables|Default|SetWorldRipInProgress false)
    (Development|PrintString "WorldRip Finished!")
    (Development|PrintString (Utilities|String|ToString(Rotator) (Math|Rotator|MakeRotfromZ (Variables|Default|GetTargetUp))) true true "(R=0.000000,G=0.660000,B=1.000000,A=1.000000)" 1e+01)))

(event EventTick
  (params (DeltaSeconds :type Float%20%28single-precision%29))
  ;[1 1 1] Move Destination Camera with the player's movements during WorldRip Procedure
  (if (Variables|Default|GetWorldRipInProgress)
    (Transformation|SetWorldLocationAndRotation (Variables|Default|GetWorldRipCubeCapture) (+ (+ (Variables|Default|GetTargetLocation) (* (Variables|Default|GetTargetUp) 0.0)) (* (- (Transformation|GetWorldLocation (Variables|Default|GetCapsuleComponent)) (Variables|Default|GetActivationLocation)) (Utilities| (- (Utilities| (Variables|Default|GetTargetUp)) "1.000000,1.000000,1.000000")))) "0, 0, 0" false true)))

(event EventBeginPlay)