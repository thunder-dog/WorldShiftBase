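; WorldShiftManager is an area actor holding CanShift and CanUnshift flags that describe whether world shifting and unshifting are allowed there.
; GetShiftables returns both flags to callers.
; Overlap logic meant to copy the flags to PlayerDummy on entry and clear them on exit is disconnected from its events, so it never runs.
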(event EventBeginPlay)

(event EventActorBeginOverlap
  (params (OtherActor :type Actor%20Object%20Reference)))

(event EventTick
  (params (DeltaSeconds :type Float%20%28single-precision%29)))

(event Collision|EventActorBeginOverlap
  (params (OtherActor :type Actor%20Object%20Reference))
  ;[1 1 1] Set player's capability to shift and unshift based on variables set here
)

(event Collision|EventActorEndOverlap
  (params (OtherActor :type Actor%20Object%20Reference))
  ;[1 1 1] Ensure player can't Worldshift when they exit the area
)

(fn ConstructionScript)

(fn GetShiftables
  (return (Variables|Default|GetCanShift) (Variables|Default|GetCanUnshift)))